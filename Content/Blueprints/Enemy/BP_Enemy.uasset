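; BP_Enemy is a sprite-based patrolling enemy that walks back and forth and explodes when destroyed.
; Tick adds delta-time-scaled movement input along the actor's forward vector.
; TurnAround flips the actor 180 degrees when LedgeDetector loses overlap or WallDetector begins one, keeping it between ledges and walls.
; On Destroyed, SpawnExplosion spawns BP_Explosion at the sprite's location and rotation.
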(event OnComponentEndOverlap(LedgeDetector)
  (params (OverlappedComponent :type Primitive%20Component%20Object%20Reference) (OtherActor :type Actor%20Object%20Reference) (OtherComp :type Primitive%20Component%20Object%20Reference) (OtherBodyIndex :type Integer))
  (CallFunction|TurnAround))

(event OnComponentBeginOverlap(WallDetector)
  (params (OverlappedComponent :type Primitive%20Component%20Object%20Reference) (OtherActor :type Actor%20Object%20Reference) (OtherComp :type Primitive%20Component%20Object%20Reference) (OtherBodyIndex :type Integer) (bFromSweep :type Boolean) (SweepResult :type Hit%20Result%20Structure%20%28by%20ref%29))
  (CallFunction|TurnAround))

(event EventDestroyed
  (CallFunction|SpawnExplosion))

(event EventTick
  (params (DeltaSeconds :type Float%20%28single-precision%29))
  (Pawn|Input|AddMovementInput (Transformation|GetActorForwardVector) (* (Utilities|Time|GetWorldDeltaSeconds) 2e+01) false))

(fn ConstructionScript)

(fn TurnAround
  (Transformation|SetActorRotation (Math|Rotator|CombineRotators (Transformation|GetActorRotation) "0.000000,180.000000,0.000000")))

(fn SpawnExplosion
  (bind _sprite (Variables|Default|GetSprite))
  (bind _returnvalue (Transformation|GetWorldTransform _sprite))
  (Game|SpawnActorfromClass "/Game/Blueprints/BP_Explosion.BP_Explosion_C" (Math|Transform|MakeTransform (.location _returnvalue) (.rotation _returnvalue) "1.000000,1.000000,1.000000") "Undefined" "MultiplyWithRoot" 0 0))